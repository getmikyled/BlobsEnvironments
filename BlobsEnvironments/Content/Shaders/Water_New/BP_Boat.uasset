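; Boat actor that hands its pontoon points to a Niagara buoyancy system and visualizes the results it gets back.
; On BeginPlay it registers itself as the system's Blueprint callback, pushes the Pontoons vector array, then reinitializes the system.
; Exported particle data returns through ParticleData, which only draws debug lines from each position along its velocity; no forces are applied to the boat here.
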(event `self.ReceiveBeginPlay`
  (bind _ns_buoyancy (`self.NS_Buoyancy`))
  (`NiagaraComponent.SetVariableObject` _ns_buoyancy "Blueprint" self)
  (`NiagaraDataInterfaceArrayFunctionLibrary.SetNiagaraArrayVector` _ns_buoyancy "Pontoons" (`self.Pontoons`))
  (`NiagaraComponent.ReinitializeSystem` _ns_buoyancy))

(event `self.ReceiveParticleData`
  (params (Data :type "Array of BasicParticleData Structure (by ref)") (NiagaraSystem :type "NiagaraSystem Object Reference") (SimulationPositionOffset :type "Vector Structure (by ref)"))
  (for _array_element Data
    (bind (_position _size _velocity) (break `BasicParticleData` _array_element))
    (`KismetSystemLibrary.DrawDebugLine` _position (+ _position _velocity) (struct :`R` 1.0 :`G` 0.182886 :`B` 0.126476 :`A` 1.0) 0.0 4.0)))

(fn `UserConstructionScript`)